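; AK-47 gun Blueprint, used as a child actor of a ShooterAI to fire at the player.
; StartShooting and StopShooting toggle a firing flag that Tick checks, using a short Delay to throttle calls to FireBullet.
; FireBullet casts the parent actor to ShooterAI and spawns an actor at that AI's location, rotated toward the first player's pawn.
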(event Custom|StartShooting
  (Variables|Default|SetIsFiring true))

(event Custom|StopShooting
  (Variables|Default|SetIsFiring false))

(event EventBeginPlay)

(event Collision|EventActorBeginOverlap
  (params (OtherActor :type Actor%20Object%20Reference)))

(event EventTick
  (params (DeltaSeconds :type Float%20%28single-precision%29))
  (if (Variables|Default|GetIsFiring)
    (Utilities|FlowControl|Delay 0.2)
    (CallFunction|FireBullet)))

(fn ConstructionScript)

(fn FireBullet
  (bind _asshooter_ai (Utilities|Casting|CastToShooterAI (Actor|GetParentActor)))
  (Game|SpawnActorfromClass "/Game/Game/BluePrints/Gun_V1/Bullet.Bullet_C" (Math|Transform|MakeTransform (Transformation|GetActorLocation _asshooter_ai) (Math|Rotator|FindLookatRotation (Transformation|GetActorLocation _asshooter_ai) (Transformation|GetWorldLocation (Variables|/Script/Engine.Actor|GetRootComponent (Game|Player|GetPlayerPawn 0))))) "Undefined" 0 0))