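; NPC Blueprint that roams at random and can show an indicator cube when interested in a deal.
; Two seconds after BeginPlay, a coin flip decides between moving to a random reachable point within a short radius and idling.
; After each move, failed move or idle, it waits briefly and repeats while CanMove is true.
; The DealInterested event makes the Cube and its children visible.
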(event Custom|DealInterested
  (Rendering|SetVisibility (Variables|Default|GetCube) true true))

(event EventBeginPlay
  (Utilities|FlowControl|Delay 2.0)
  ;[1 1 1] Very very basic AI roaming
  (Utilities|FlowControl|Sequence :!label _label
    (:then_0
      (Variables|Default|SetMoving%20? (Math|Random|RandomBool)))
    (:then_1
      (if (Variables|Default|GetMoving%20?)
        (AI|AIMoveTo (Class|PawnMovementComponent|GetPawnOwner (Variables|Character|GetCharacterMovement)) (.RandomLocation (AI|Navigation|GetRandomReachablePointinRadius (Transformation|GetActorLocation self) 2e+02 0 0)) 0 5.0 false
          (:OnSuccess
            _)
          (:OnFail
            _)))
      (Utilities|FlowControl|Delay 1.0)
      (if (Variables|Default|GetCanMove?)
        (goto _label)))))

(fn ConstructionScript)