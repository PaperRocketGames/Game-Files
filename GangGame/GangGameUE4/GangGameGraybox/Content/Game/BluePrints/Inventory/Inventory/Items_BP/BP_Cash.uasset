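; BP_Cash is a cash pickup that adds a small random amount of money to the player on overlap.
; When a CharacterMain enters its collision box, it sets that character's MainCollidingWithEnum.
; It then adds the random amount to player 0's PlayerMoney, rounds the total to a whole number and destroys itself.
; The money goes to player 0's character, whichever CharacterMain triggered the overlap.
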(event OnComponentBeginOverlap(CollisionBox)
  (params (OverlappedComponent :type Primitive%20Component%20Object%20Reference) (OtherActor :type Actor%20Object%20Reference) (OtherComp :type Primitive%20Component%20Object%20Reference) (OtherBodyIndex :type Integer) (bFromSweep :type Boolean) (SweepResult :type Hit%20Result%20Structure%20%28by%20ref%29))
  (bind _ascharacter_main (Utilities|Casting|CastToCharacterMain OtherActor))
  (Variables|/Game/TopDownBP/Blueprints/CharacterMain.CharacterMain_C|SetMainCollidingWithEnum _ascharacter_main "NewEnumerator4")
  (bind _ascharacter_main_2 (Utilities|Casting|CastToCharacterMain (Game|GetPlayerCharacter 0)))
  (Variables|/Game/TopDownBP/Blueprints/CharacterMain.CharacterMain_C|SetPlayerMoney _ascharacter_main_2 (Math|Conversions|ToFloat(Integer) (Math|Float|Round (+ (Variables|/Game/TopDownBP/Blueprints/CharacterMain.CharacterMain_C|GetPlayerMoney _ascharacter_main_2) (Math|Random|RandomFloatinRange 1.0 5.0)))))
  (Actor|DestroyActor))

(fn ConstructionScript
  (|CallParentFunction))