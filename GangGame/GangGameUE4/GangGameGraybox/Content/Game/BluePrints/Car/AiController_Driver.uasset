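; AI controller that drives a BP_Vehicle_V2 along spline road paths.
; While its Tick gate is open, it chases a target point that advances along the spline at car speed plus an offset, only while the car is near it.
; Yaw to the target sets steering and scales throttle with distance, drawing a debug line.
; At spline end it switches to the path's next spline, or zeroes inputs if none exists.
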(event Custom|StartDriving
  (Utilities|FlowControl|Gate true) ; enters at Open
)

(event Custom|NewPath
  (params (NewRoad :type BP%20Road%20Spline%20Object%20Reference))
  (bind _controlledcar (Variables|Default|GetControlledCar))
  (bind _vehiclemovement (Variables|/Script/PhysXVehicles.WheeledVehicle|GetVehicleMovement _controlledcar))
  (Utilities|IsValid NewRoad
    (:Is%20Valid
      (Variables|Default|SetRecentlyChangedPaths true)
      (CallFunction|SetupSpline NewRoad)
      (Utilities|FlowControl|Delay 4.0)
      (Variables|Default|SetRecentlyChangedPaths false))
    (:Is%20Not%20Valid
      (Variables|Default|SetCurrentPath 0)
      (Utilities|FlowControl|Delay 0.2)
      (Class|WheeledVehicleMovementComponent|SetSteeringInput _vehiclemovement 0.0)
      (Class|WheeledVehicleMovementComponent|SetThrottleInput _vehiclemovement 0.0))))

(event Custom|StopDriving
  (Utilities|FlowControl|Gate true) ; enters at Close
)

(event EventBeginPlay
  (bind _controlledcar (Variables|Default|GetControlledCar))
  (bind _currentpath (Variables|/Game/Game/BluePrints/Car/BP_Vehicle_V2.BP_Vehicle_V2_C|GetCurrentPath _controlledcar))
  (CallFunction|GetPawn)
  (Utilities|IsValid _currentpath
    (:Is%20Valid
      (CallFunction|SetupSpline _currentpath))))

(event EventTick
  (params (DeltaSeconds :type Float%20%28single-precision%29))
  (Utilities|FlowControl|Gate true
    (:Exit
      (CallFunction|Drive))))

(fn ConstructionScript)

(fn GetPawn
  (bind _asbp_vehicle_v2 (Utilities|Casting|CastToBP_Vehicle_V2 (Pawn|GetControlledPawn)))
  (bind _output_get (Variables|Default|SetControlledCar _asbp_vehicle_v2))
  (Utilities|IsValid _output_get
    (:Is%20Valid
      (CallFunction|StartDriving))))

(fn Drive
  (Utilities|IsValid (Variables|Default|GetCurrentPath)
    (:Is%20Valid
      (CallFunction|SplineDrive))))

(fn Steering
  (bind _controlledcar (Variables|Default|GetControlledCar))
  (bind _splineposition (Variables|Default|GetSplinePosition))
  (bind _returnvalue (Transformation|GetActorLocation _controlledcar))
  (bind _returnvalue_2 (Transformation|GetActorTransform _controlledcar))
  (bind _returnvalue_3 (Math|Rotator|FindLookatRotation _returnvalue _splineposition))
  (bind _returnvalue_4 (Math|Rotator|GetRotationXVector _returnvalue_3))
  (bind _returnvalue_5 (Math|Transform|InverseTransformDirection _returnvalue_2 _returnvalue_4))
  (bind _returnvalue_6 (Math|Conversions|RotationFromXVector _returnvalue_5))
  (bind _output_get (LocalVariables|SetSteeringToApply (Math|Float|MapRangeClamped (.yaw _returnvalue_6) -1.8e+02 1.8e+02 -1.5 1.5)))
  (Class|WheeledVehicleMovementComponent|SetSteeringInput (Variables|/Script/PhysXVehicles.WheeledVehicle|GetVehicleMovement (Variables|Default|GetControlledCar)) _output_get)
  (return (* -1 (Math|Float|MapRangeClamped (Math|Float|Absolute(Float) (.yaw _returnvalue_6)) 0.0 25.0 -1.0 -0.25))))

(fn GetSplinePosition
  (bind (_newdistance _splinevalid) (CallFunction|GetDistanceAlongSpline))
  (bind _currentpath (Variables|Default|GetCurrentPath))
  (bind _spline (Variables|/Game/Game/BluePrints/Car/Traffic/BP_RoadSpline.BP_RoadSpline_C|GetSpline _currentpath))
  (bind _returnvalue (Spline|GetLocationatDistanceAlongSpline _spline _newdistance "World"))
  (if _splinevalid
    (Rendering|Debug|DrawDebugLine (Transformation|GetActorLocation (Variables|Default|GetControlledCar)) _returnvalue "(R=1.000000,G=0.042000,B=0.000000,A=1.000000)" 0.0 25.0)
    (return _returnvalue)
    (else
      (return "0, 0, 0"))))

(fn SplineDrive
  (Variables|Default|SetSplinePosition (CallFunction|GetSplinePosition))
  (bind _throttlemultiplier (CallFunction|Steering))
  (bind _output_get (Variables|Default|SetCurrentThrottleInput (* _throttlemultiplier (Math|Float|MapRangeClamped (Math|Vector|VectorLength (- (Transformation|GetActorLocation (Variables|Default|GetControlledCar)) (Variables|Default|GetSplinePosition))) 3e+02 6e+02 0.0 1.0))))
  (Class|WheeledVehicleMovementComponent|SetThrottleInput (Variables|/Script/PhysXVehicles.WheeledVehicle|GetVehicleMovement (Variables|Default|GetControlledCar)) _output_get))

(fn GetDistanceAlongSpline
  (bind _currentpath (Variables|Default|GetCurrentPath))
  (Utilities|IsValid _currentpath
    (:Is%20Valid
      (bind _output_get (Variables|Default|SetDistanceAlongCurrentSpline (Math|Float|SelectFloat (Math|Interpolation|FInterptoConstant (Variables|Default|GetDistanceAlongCurrentSpline) (Variables|Default|GetCurrentSplineLength) (Utilities|Time|GetWorldDeltaSeconds) (+ (Math|Vector|VectorLength (Transformation|GetVelocity (Variables|Default|GetControlledCar))) 35.0)) (Variables|Default|GetDistanceAlongCurrentSpline) (<= (Math|Vector|VectorLength (- (Transformation|GetActorLocation (Variables|Default|GetControlledCar)) (Spline|GetLocationatDistanceAlongSpline (Variables|/Game/Game/BluePrints/Car/Traffic/BP_RoadSpline.BP_RoadSpline_C|GetSpline (Variables|Default|GetCurrentPath)) (Variables|Default|GetDistanceAlongCurrentSpline) "World"))) (Variables|Default|GetDistanceToPushSpline)))))
      (if (>= _output_get (Variables|Default|GetCurrentSplineLength))
        (bind _output (Default|GetNextSpline _currentpath))
        (Utilities|IsValid _output
          (:Is%20Valid
            (CallFunction|NewPath _output)
            (return 0.0 false))
          (:Is%20Not%20Valid
            (CallFunction|NewPath)
            (return 0.0 false)))
        (else
          (return _output_get true))))
    (:Is%20Not%20Valid
      (return 0.0 true))))

(fn SetupSpline
  (params (CurrentPath :type BP%20Road%20Spline%20Object%20Reference))
  (Utilities|IsValid CurrentPath
    (:Is%20Valid
      (Variables|Default|SetCurrentPath CurrentPath))
    (:Is%20Not%20Valid
      (Utilities|IsValid (Variables|Default|GetCurrentPath)
        (:Is%20Valid
          _))))
  (Variables|Default|SetCurrentSplineLength (Spline|GetSplineLength (Variables|/Game/Game/BluePrints/Car/Traffic/BP_RoadSpline.BP_RoadSpline_C|GetSpline (Variables|Default|GetCurrentPath))))
  (Variables|Default|SetDistanceAlongCurrentSpline 0.0))