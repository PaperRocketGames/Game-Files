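; Traffic vehicle Blueprint, apparently a child of BP_Veh_1, that lets the player take control of it by pointing at it.
; Mesh cursor-over events set and clear a Cursor flag.
; Tick polls the E key on player controller 0 while the flag is set, and that controller possesses the vehicle when the key is down.
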(event OnBeginCursorOver(Mesh)
  (params (TouchedComponent :type Primitive%20Component%20Object%20Reference))
  (Variables|Default|SetCursor true))

(event OnEndCursorOver(Mesh)
  (params (TouchedComponent :type Primitive%20Component%20Object%20Reference))
  (Variables|Default|SetCursor false))

(event EventBeginPlay)

(event Collision|EventActorBeginOverlap
  (params (OtherActor :type Actor%20Object%20Reference)))

(event EventTick
  (params (DeltaSeconds :type Float%20%28single-precision%29))
  (if (and (Variables|Default|GetCursor) (Game|Player|IsInputKeyDown (Game|GetPlayerController 0) "E"))
    (Pawn|Possess (Game|GetPlayerController 0) self)))

(fn ConstructionScript)