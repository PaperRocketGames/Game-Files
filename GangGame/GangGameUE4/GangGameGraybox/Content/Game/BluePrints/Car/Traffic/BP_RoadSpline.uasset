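; BP_RoadSpline is a road segment Blueprint in the car traffic system that supplies a following spline through GetNextSpline.
; It references Straight, RightTurn and LeftTurn connections, with GetRandomSpline rebuilding the ValidSplines array on each call.
; Only when Straight is invalid does it gather valid turns and return one at random.
; A valid Straight is added to the array, but that branch ends without returning it.
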(event EventBeginPlay)

(event Collision|EventActorBeginOverlap
  (params (OtherActor :type Actor%20Object%20Reference)))

(event EventTick
  (params (DeltaSeconds :type Float%20%28single-precision%29)))

(fn ConstructionScript)

(fn GetNextSpline
  (bind _output (CallFunction|GetRandomSpline))
  (return _output))

(fn GetRandomSpline
  (bind _straight (Variables|Default|GetStraight))
  (bind _rightturn (Variables|Default|GetRightTurn))
  (bind _leftturn (Variables|Default|GetLeftTurn))
  (bind _validsplines (Variables|Default|GetValidSplines))
  (Utilities|Array|Clear (Variables|Default|GetValidSplines))
  (Utilities|IsValid _straight
    (:Is%20Valid
      (Utilities|Array|AddUnique (Variables|Default|GetValidSplines) _straight))
    (:Is%20Not%20Valid
      (Utilities|IsValid _rightturn
        (:Is%20Valid
          (Utilities|Array|AddUnique (Variables|Default|GetValidSplines) _rightturn))
        (:Is%20Not%20Valid
          _))
      (Utilities|IsValid _leftturn
        (:Is%20Valid
          (Utilities|Array|AddUnique (Variables|Default|GetValidSplines) _leftturn))
        (:Is%20Not%20Valid
          _))
      (if (Utilities|Array|IsValidIndex _validsplines)
        (return (Utilities|Array|Get(acopy) _validsplines (Math|Random|RandomIntegerinRange 0 (Utilities|Array|LastIndex _validsplines))))
        (else
          (return 0))))))