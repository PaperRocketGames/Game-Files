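; Street lamp actor from the PolygonTown set with two point lights and a spot light that can be switched on and off.
; TurnOnLights and TurnOffLights toggle the lamp by setting fixed intensities or zero on all three lights, rather than changing visibility.
; The event graph and construction script are empty, so nothing in this Blueprint calls either function.
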(event EventBeginPlay)

(event Collision|EventActorBeginOverlap
  (params (OtherActor :type Actor%20Object%20Reference)))

(event EventTick
  (params (DeltaSeconds :type Float%20%28single-precision%29)))

(fn ConstructionScript)

(fn TurnonLights
  (Rendering|Components|Light|SetIntensity (Variables|Default|GetPointLight1) 1e+04)
  (Rendering|Components|Light|SetIntensity (Variables|Default|GetSpotLight) 2e+04))

(fn TurnOffLights
  (Rendering|Components|Light|SetIntensity (Variables|Default|GetPointLight1) 0.0)
  (Rendering|Components|Light|SetIntensity (Variables|Default|GetSpotLight) 0.0))